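; Snake hazard actor that hurts the side-scrolling player character on contact.
; On BeginPlay it rotates itself once to face the player pawn using a look-at rotation; Tick is empty, so it does not keep tracking.
; Actor overlap casts to BP_SideScrollingCharacter and calls its TakeDamage.
; Unconnected physics, force and SnakeCobra component rotation nodes remain in the graph but never run.
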(event `LookAtPlayer`
  (bind (_returnvalue_x _returnvalue_y _returnvalue_z) (`KismetMathLibrary.BreakVector` (`self.K2_GetActorLocation`)))
  (bind (_returnvalue_x_2 _returnvalue_y_2 _returnvalue_z_2) (`KismetMathLibrary.BreakVector` (`self.K2_GetActorLocation` (`GameplayStatics.GetPlayerPawn` 0))))
  (`self.K2_SetActorRotation` (`KismetMathLibrary.FindLookAtRotation` (`KismetMathLibrary.MakeVector` _returnvalue_x _returnvalue_y _returnvalue_z) (`KismetMathLibrary.MakeVector` _returnvalue_x_2 _returnvalue_y_2 _returnvalue_z_2))))

(event `self.ReceiveBeginPlay`
  (`self.LookAtPlayer`))

(event `self.ReceiveTick`
  (params (DeltaSeconds :type "Float (single-precision)")))

(event `self.ReceiveActorBeginOverlap`
  (params (OtherActor :type "Actor Object Reference"))
  (bind _asbp_side_scrolling_character (cast `/Game/Variant_SideScrolling/Blueprints/BP_SideScrollingCharacter` OtherActor))
  (`SideScrollingCharacter.TakeDamage` _asbp_side_scrolling_character 1.0 (`self.Damage Event`) null null))

(fn `UserConstructionScript`)