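; BP_SnakeBasket is a breakable basket that shatters through Chaos Destruction when it dies.
; Its Die override runs the parent logic, then spawns an FS_MasterField Field System actor, configures it and triggers it.
; With a valid damage causer, the field is nudged toward the attacker and uses a stronger radial magnitude, otherwise it fires weaker at the basket's location.
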(fn `Die`
  (params (DamageCauser :type "Actor Object Reference"))
  (locals (FSMasterFieldLocation :type "Vector Structure"))
  (bind _returnvalue (`KismetSystemLibrary.IsValid` DamageCauser))
  (set `local.FSMasterFieldLocation` (`self.K2_GetActorLocation`))
  (if _returnvalue
    (set `local.FSMasterFieldLocation` (+ (`local.FSMasterFieldLocation`) (* 10.0 (`KismetMathLibrary.Normal` (- (`self.K2_GetActorLocation` DamageCauser) (`SceneComponent.K2_GetComponentLocation` (`self.SphereComp`))))))) ; 相手がいる場合は、FS をその方向に少し寄せる
  )
  (`parent.Die` null)
  (bind _returnvalue_2 (`|SpawnActorFromClass` "/Engine/EditorResources/FieldNodes/FS_MasterField.FS_MasterField_C" (`KismetMathLibrary.MakeTransform` (`local.FSMasterFieldLocation`) (`self.K2_GetActorRotation`)) "Undefined" "MultiplyWithRoot" null null)) ; Chaos Destruction を発生させるための Field System を発動する
  (set `/Engine/EditorResources/FieldNodes/FS_MasterField.ActivationType` "NewEnumerator4" _returnvalue_2)
  (if _returnvalue
    (set `/Engine/EditorResources/FieldNodes/FS_MasterField.Radial Magnitude` 300.0 _returnvalue_2)
    (else
      (set `/Engine/EditorResources/FieldNodes/FS_MasterField.Radial Magnitude` 100.0 _returnvalue_2)))
  (`/Engine/EditorResources/FieldNodes/FS_MasterField.CE_Trigger` _returnvalue_2))

(fn `UserConstructionScript`
  (`parent.UserConstructionScript`))