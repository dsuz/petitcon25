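; Base enemy Blueprint for a side-scroller, implementing the Hugger humanoid type that walks at the player and grabs them.
; While alive and not hugging, Tick feeds movement input toward the player pawn.
; On hit, a grounded player or an already-hugging enemy triggers a one-time Hug that stops the chase and calls Hug on the player, so grabs chain through touching enemies.
; Helper functions classify actors and query hug state.
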(event `self.ReceiveTick`
  (params (DeltaSeconds :type "Float (single-precision)"))
  ; 生きていてつかみモードじゃなければプレイヤーの方に歩く
  (if (`|EnumEquality` (`self.HumanoidEnemyType`) "Hugger")
    (if (and (> (`self.Life`) 0.0) (not (`self.bIsHugging`)))
      (`self.MoveToPlayer`))))

(event `MoveToPlayer`
  ; プレイヤーの方に歩く
  (`PawnMovementComponent.AddInputVector` (`self.CharacterMovement`) (`KismetMathLibrary.Normal` (- (`self.K2_GetActorLocation` (`GameplayStatics.GetPlayerPawn` 0)) (`self.K2_GetActorLocation`))) false))

(event `self.ReceiveHit`
  (params (MyComp :type "PrimitiveComponent Object Reference") (Other :type "Actor Object Reference") (OtherComp :type "PrimitiveComponent Object Reference") (bSelfMoved :type Boolean) (HitLocation :type "Vector Structure") (HitNormal :type "Vector Structure") (NormalImpulse :type "Vector Structure") (Hit :type "HitResult Structure (by ref)"))
  ; つかみを判定する
  (if (`|EnumEquality` (`self.HumanoidEnemyType`) "Hugger")
    (if (`self.IsPlayerOnTheGround` Other)
      (`/Engine/EditorBlueprintResources/StandardMacros.DoOnce` false :!label _label
        (:`Completed`
          (`self.Hug`)))
      (elif (`self.IsHuggingEnemy` Other)
        (goto _label)))))

(event `Hug`
  ; つかむ
  (set `self.bIsHugging` true)
  (bind _asside_scrolling_character (cast `SideScrollingCharacter` (`GameplayStatics.GetPlayerPawn` 0)))
  (`SideScrollingCharacter.Hug` _asside_scrolling_character))

(fn `IsEnemy`
  (params (Actor :type "Actor Object Reference"))
  (returns (ReturnValue :type Boolean))
  (cast `Enemy` Actor
    (:`then`
      (return true))
    (:`CastFailed`
      (return false))))

(fn `IsHuggingEnemy`
  (params (Actor :type "Actor Object Reference"))
  (returns (ReturnValue :type Boolean))
  (bind _asenemy (cast `Enemy` Actor)
    (:`then`
      (return (`Enemy.bIsHugging` _asenemy)))
    (:`CastFailed`
      (return false))))

(fn `IsPlayerHugged`
  (returns (ReturnValue :type Boolean))
  (bind _asside_scrolling_character (cast `SideScrollingCharacter` (`GameplayStatics.GetPlayerPawn` 0))
    (:`then`
      (bind _returnvalue (`SideScrollingCharacter.IsHugged` _asside_scrolling_character))
      (return _returnvalue))
    (:`CastFailed`
      (return false))))

(fn `IsPlayerOnTheGround`
  (params (Actor :type "Actor Object Reference"))
  (returns (ReturnValue :type Boolean))
  (bind _asside_scrolling_character (cast `SideScrollingCharacter` Actor)
    (:`then`
      (return (not (`NavMovementComponent.IsFalling` (`Character.CharacterMovement` _asside_scrolling_character)))))
    (:`CastFailed`
      (return false))))

(fn `IsPlayerOrEnemy`
  (params (Actor :type "Actor Object Reference"))
  (returns (Value :type Boolean))
  (locals (ReturnValue :type Boolean))
  (if (> (`self.Life`) 0.0)
    (cast `SideScrollingCharacter` Actor
      (:`then`
        (set `local.ReturnValue` true :!label _label))
      (:`CastFailed`
        (cast `Enemy` Actor
          (:`then`
            (goto _label))
          (:`CastFailed`
            _)))))
  (return (`local.ReturnValue`)))

(fn `UserConstructionScript`)