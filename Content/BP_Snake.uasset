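; BP_Snake is a hazard actor that charges along the X axis and damages the side-scrolling character on overlap.
; At BeginPlay it locks its facing and direction toward the player's X position, without updating them afterward.
; Each tick it applies that rotation to Pivot and pushes Box with a mass-independent force scaled by Speed.
; After each hit and a short delay, Speed is multiplied, so repeated overlaps compound the acceleration.
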(event `self.ReceiveBeginPlay`
  (set `self.TargetRotation` (`self.GetTargetRotation`))
  (set `self.TargetDirection` (`self.GetTargetDirection`)))

(event `self.ReceiveTick`
  (params (DeltaSeconds :type "Float (single-precision)"))
  (`SceneComponent.K2_SetWorldRotation` (`self.Pivot`) (`self.TargetRotation`) false false)
  (`PrimitiveComponent.AddForce` (`self.Box`) (* (`self.TargetDirection`) (`self.Speed`)) "None" true))

(event `self.ReceiveActorBeginOverlap`
  (params (OtherActor :type "Actor Object Reference"))
  (bind _asbp_side_scrolling_character (cast `/Game/Variant_SideScrolling/Blueprints/BP_SideScrollingCharacter` OtherActor))
  (`SideScrollingCharacter.TakeDamage` _asbp_side_scrolling_character (`self.Damage`) (`self.Damage Event`) null null)
  (`KismetSystemLibrary.Delay` 0.2)
  (set `self.Speed` (* (`self.Speed`) 5.0)))

(fn `GetTargetDirection`
  (returns (Return :type "Vector Structure"))
  (bind _returnvalue_x (`KismetMathLibrary.BreakVector` (`self.K2_GetActorLocation`)))
  (bind _returnvalue_x_2 (`KismetMathLibrary.BreakVector` (`self.K2_GetActorLocation` (`GameplayStatics.GetPlayerPawn` 0))))
  (return (`KismetMathLibrary.Normal` (- (`KismetMathLibrary.MakeVector` _returnvalue_x_2) (`KismetMathLibrary.MakeVector` _returnvalue_x)))))

(fn `GetTargetRotation`
  (returns (Return :type "Rotator Structure"))
  (bind _returnvalue_x (`KismetMathLibrary.BreakVector` (`self.K2_GetActorLocation`)))
  (bind _returnvalue_x_2 (`KismetMathLibrary.BreakVector` (`self.K2_GetActorLocation` (`GameplayStatics.GetPlayerPawn` 0))))
  (return (`KismetMathLibrary.FindLookAtRotation` (`KismetMathLibrary.MakeVector` _returnvalue_x) (`KismetMathLibrary.MakeVector` _returnvalue_x_2))))

(fn `UserConstructionScript`)