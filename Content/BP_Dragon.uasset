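; BP_Dragon is a side-scroller enemy that appears in smoke, turns toward the player and drops under physics until its mesh registers a hit, which freezes it in place.
; Attack damages every BP_SideScrollingCharacter overlapping AttackZone.
; Any damage while Damagable destroys it in a smoke puff; BecomeInvincible clears that flag.
; Facing uses only X positions, and nothing here calls Attack or BecomeInvincible.
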(event `BecomeInvincible`
  ; 無敵化
  (set `self.Damagable` false) ; もう倒せない
)

(event `LookAtPlayer`
  (bind _returnvalue_x (`KismetMathLibrary.BreakVector` (`self.K2_GetActorLocation`)))
  (bind _returnvalue_x_2 (`KismetMathLibrary.BreakVector` (`self.K2_GetActorLocation` (`GameplayStatics.GetPlayerPawn` 0))))
  ; プレイヤーの方に向ける
  (`self.K2_SetActorRotation` (`KismetMathLibrary.FindLookAtRotation` (`KismetMathLibrary.MakeVector` _returnvalue_x) (`KismetMathLibrary.MakeVector` _returnvalue_x_2))))

(event `Attack`
  ; 攻撃
  (for _array_element (`PrimitiveComponent.GetOverlappingActors` (`self.AttackZone`) "/Game/Variant_SideScrolling/Blueprints/BP_SideScrollingCharacter.BP_SideScrollingCharacter_C")
    (bind _asbp_side_scrolling_character (cast `/Game/Variant_SideScrolling/Blueprints/BP_SideScrollingCharacter` _array_element))
    (`SideScrollingCharacter.TakeDamage` _asbp_side_scrolling_character (`self.Damage`) (`self.Damage Event`) null null)))

(event `self.ReceiveBeginPlay`
  ; 登場
  (`self.Smoke` false)
  (`self.LookAtPlayer`)
  (`PrimitiveComponent.SetSimulatePhysics` (`self.BoxCollision`) true))

(event `self.SkeletalMesh.OnComponentHit`
  (params (HitComponent :type "PrimitiveComponent Object Reference") (OtherActor :type "Actor Object Reference") (OtherComp :type "PrimitiveComponent Object Reference") (NormalImpulse :type "Vector Structure") (Hit :type "HitResult Structure (by ref)"))
  ; 登場して着地したら、固定する
  (`PrimitiveComponent.SetSimulatePhysics` (`self.BoxCollision`) false) ; 体当たりしても動かないように
)

(event `self.ReceiveAnyDamage`
  (params (Damage :type "Float (single-precision)") (DamageType :type "DamageType Object Reference") (InstigatedBy :type "Controller Object Reference") (DamageCauser :type "Actor Object Reference"))
  ; 攻撃を食らったとき
  (if (`self.Damagable`)
    (`self.Smoke` true)))

(event `Smoke`
  (params (IsDestoy :type Boolean))
  ; 煙幕をはる
  (`|SpawnActorFromClass` (`self.SmokeEffect`) (`KismetMathLibrary.MakeTransform` (`SceneComponent.K2_GetComponentLocation` (`self.Center`)) (struct) (7.0 7.0 7.0)) "Undefined" "MultiplyWithRoot" null null)
  (if IsDestoy
    (`self.K2_DestroyActor`)))

(fn `UserConstructionScript`)