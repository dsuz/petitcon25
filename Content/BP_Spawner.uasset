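; BP_Spawner is a spawner actor that creates instances of a configurable class at its own transform.
; When active, it spawns once on BeginPlay and, if Repeat is set, keeps spawning via a Tick-driven timer.
; The interval is re-randomized between min and max after each spawn.
; Spawns ignore collisions, and any spawned Pawn receives its default controller.
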(event `MySpawn`
  (bind _returnvalue (`|SpawnActorFromClass` (`self.ActorSpawned`) (`self.GetTransform`) "AlwaysSpawn" "MultiplyWithRoot" null null))
  (bind _aspawn (cast `Pawn` _returnvalue))
  (`Pawn.SpawnDefaultController` _aspawn))

(event `SetRandomInterval`
  (set `self.Interval` (`KismetMathLibrary.RandomFloatInRange` (`self.IntervalMin`) (`self.IntervalMax`))))

(event `self.ReceiveBeginPlay`
  (if (`self.Active`)
    (`self.SetRandomInterval`)
    (if (not (`self.Repeat`))
      (set `self.Active` false))
    (`self.MySpawn` :!label _label)
    (set `self.Timer` 0.0)
    (`self.SetRandomInterval`)))

(event `self.ReceiveTick`
  (params (DeltaSeconds :type "Float (single-precision)"))
  (if (`self.Active`)
    (bind _output_get (set `self.Timer` (+ DeltaSeconds (`self.Timer`))))
    (if (> _output_get (`self.Interval`))
      (goto _label))))

(fn `UserConstructionScript`)